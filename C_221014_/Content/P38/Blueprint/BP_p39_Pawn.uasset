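; Player-controlled P-38 plane pawn that flies constantly forward and spins its left and right propellers every frame.
; Tick feeds the actor's forward vector into movement input for FloatingPawnMovement, replacing an unused manual local-offset move.
; Roll and Pitch axes apply clamped, delta-time-scaled local rotations, so steering redirects the flight path.
; Holding Boost raises the movement component's max speed, and releasing it restores the slower speed.
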(event `self.ReceiveTick`
  (params (DeltaSeconds :type "Float (single-precision)"))
  ;[1 1 1] Left Rotate
  (`SceneComponent.K2_AddLocalRotation` (`self.Left`) (`KismetMathLibrary.MakeRotator` (* (`self.PropellerRotationSpeed`) (`GameplayStatics.GetWorldDeltaSeconds`))) false false)
  ;[1 1 1] Right Rotate
  (`SceneComponent.K2_AddLocalRotation` (`self.Right`) (`KismetMathLibrary.MakeRotator` (* (`self.PropellerRotationSpeed`) (`GameplayStatics.GetWorldDeltaSeconds`))) false false)
  ;[1 1 1] 앞으로감 (월드기준임)
  (`self.AddMovementInput` (`self.GetActorForwardVector`)))

(event `InputAxis|Roll`
  (params (AxisValue :type "Float (single-precision)"))
  ;[1 1 1] X 축 회전
  (`self.K2_AddActorLocalRotation` (`KismetMathLibrary.MakeRotator` (* (`KismetMathLibrary.FClamp` AxisValue -1.0) (`self.RotationSpeed`) (`GameplayStatics.GetWorldDeltaSeconds`)))))

(event `InputAxis|Pitch`
  (params (AxisValue :type "Float (single-precision)"))
  ;[1 1 1] Y 축 회전
  (`self.K2_AddActorLocalRotation` (`KismetMathLibrary.MakeRotator` 0.0 (* (`KismetMathLibrary.FClamp` AxisValue -1.0) (`self.RotationSpeed`) (`GameplayStatics.GetWorldDeltaSeconds`)))))

(event `InputAction|Boost`
  (params (Key :type "Key Structure"))
  (:`Pressed`
    (bind _output_get (set `self.MoveSpeed` 500.0))
    (set `FloatingPawnMovement.MaxSpeed` _output_get (`self.FloatingPawnMovement`)))
  (:`Released`
    (bind _output_get_2 (set `self.MoveSpeed` 50.0))
    (set `FloatingPawnMovement.MaxSpeed` _output_get_2 (`self.FloatingPawnMovement`))))

(fn `UserConstructionScript`)