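; BP_p38 is a player-controllable P-38 aircraft that flies forward continuously along its local X axis at a set move speed.
; Tick spins the Left and Right propeller components around their roll axis and advances the actor.
; Roll and Pitch axis inputs rotate the whole actor locally.
; All motion is scaled by world delta seconds to stay consistent across machine performance.
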(event `self.ReceiveTick`
  (params (DeltaSeconds :type "Float (single-precision)"))
  ;[1 1 1] Left Rotate
  (`SceneComponent.K2_AddLocalRotation` (`self.Left`) (`KismetMathLibrary.MakeRotator` (* (`self.PropellerRotationSpeed`) (`GameplayStatics.GetWorldDeltaSeconds`))) false false)
  ;[1 1 1] Right Rotate
  (`SceneComponent.K2_AddLocalRotation` (`self.Right`) (`KismetMathLibrary.MakeRotator` (* (`self.PropellerRotationSpeed`) (`GameplayStatics.GetWorldDeltaSeconds`))) false false)
  ;[1 1 1] Move P38
  (`self.K2_AddActorLocalOffset` (`KismetMathLibrary.MakeVector` (* (`self.MoveSpeed`) (`GameplayStatics.GetWorldDeltaSeconds`)))))

(event `InputAxis|Roll`
  (params (AxisValue :type "Float (single-precision)"))
  ;[1 1 1] X 축 회전
  (`self.K2_AddActorLocalRotation` (`KismetMathLibrary.MakeRotator` (* AxisValue (`self.RotationSpeed`) (`GameplayStatics.GetWorldDeltaSeconds`)))))

(event `InputAxis|Pitch`
  (params (AxisValue :type "Float (single-precision)"))
  ;[1 1 1] Y 축 회전
  (`self.K2_AddActorLocalRotation` (`KismetMathLibrary.MakeRotator` 0.0 (* AxisValue (`self.RotationSpeed`) (`GameplayStatics.GetWorldDeltaSeconds`)))))

(fn `UserConstructionScript`)